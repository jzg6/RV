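; BP_BallRack is a bowling ball dispenser triggered by overlapping its box component.
; Overlap start lowers the sphere like a pressed button, spawns a BP_BowlingBall at the audio component's transform and plays the sound.
; The audio component doubles as launch point, its forward vector giving the new ball a mass-independent impulse.
; Overlap end raises the sphere again, with no filter on the overlapping actor.
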(event `self.Box.OnComponentBeginOverlap`
  (params (OverlappedComponent :type "PrimitiveComponent Object Reference") (OtherActor :type "Actor Object Reference") (OtherComp :type "PrimitiveComponent Object Reference") (OtherBodyIndex :type Integer) (bFromSweep :type Boolean) (SweepResult :type "HitResult Structure (by ref)"))
  (bind _sphere (`self.Sphere`))
  (bind _audio (`self.Audio`))
  (`SceneComponent.K2_SetWorldLocation` _sphere (- (`SceneComponent.K2_GetComponentLocation` _sphere) (0.0 0.0 2.0)) false false)
  (bind _returnvalue (`|SpawnActorFromClass` "/Game/BluePrints/BP_BowlingBall.BP_BowlingBall_C" (`SceneComponent.K2_GetComponentToWorld` _audio) "Undefined" "MultiplyWithRoot" null null))
  (`PrimitiveComponent.AddImpulse` (`/Game/BluePrints/BP_BowlingBall.Sphere` _returnvalue) (* (`SceneComponent.GetForwardVector` _audio) (300.0 300.0 300.0)) "None" true)
  (`AudioComponent.Play` (`self.Audio`) 0.0))

(event `self.Box.OnComponentEndOverlap`
  (params (OverlappedComponent :type "PrimitiveComponent Object Reference") (OtherActor :type "Actor Object Reference") (OtherComp :type "PrimitiveComponent Object Reference") (OtherBodyIndex :type Integer))
  (bind _sphere (`self.Sphere`))
  (`SceneComponent.K2_SetWorldLocation` _sphere (+ (`SceneComponent.K2_GetComponentLocation` _sphere) (0.0 0.0 2.0)) false false))

(fn `UserConstructionScript`)